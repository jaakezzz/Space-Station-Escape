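; BP_Hatch_01 is a hatch actor that swings open when something overlaps its Box trigger and reverses when the overlap ends.
; The Door_Slide timeline drives the relative roll of SMHatch01B.
; When the timeline finishes, it disables collision on both meshes and the Box after opening, and restores it after closing.
; The construction script applies the Material variable to both hatch meshes.
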(event `self.Box.OnComponentBeginOverlap`
  (params (OverlappedComponent :type "PrimitiveComponent Object Reference") (OtherActor :type "Actor Object Reference") (OtherComp :type "PrimitiveComponent Object Reference") (OtherBodyIndex :type Integer) (bFromSweep :type Boolean) (SweepResult :type "HitResult Structure (by ref)"))
  (bind _box (`self.Box`))
  (bind (_direction _newtrack_0) (`Timeline|Door_Slide` :!label _label)
    (:`Update`
      (`SceneComponent.K2_SetRelativeRotation` (`self.SM_Hatch_01_B`) (`KismetMathLibrary.MakeRotator` _newtrack_0) false false))
    (:`Finished`
      (switch `ETimelineDirection` _direction
        (:`Forward`
          (`PrimitiveComponent.SetCollisionEnabled` _box "NoCollision")
          (`PrimitiveComponent.SetCollisionEnabled` (`self.SM_Hatch_01_A`) "NoCollision")
          (`PrimitiveComponent.SetCollisionEnabled` (`self.SM_Hatch_01_B`) "NoCollision"))
        (:`Backward`
          (`PrimitiveComponent.SetCollisionEnabled` _box "QueryAndPhysics")
          (`PrimitiveComponent.SetCollisionEnabled` (`self.SM_Hatch_01_A`) "QueryAndPhysics")
          (`PrimitiveComponent.SetCollisionEnabled` (`self.SM_Hatch_01_B`) "QueryAndPhysics"))))))

(event `self.Box.OnComponentEndOverlap`
  (params (OverlappedComponent :type "PrimitiveComponent Object Reference") (OtherActor :type "Actor Object Reference") (OtherComp :type "PrimitiveComponent Object Reference") (OtherBodyIndex :type Integer))
  (goto _label :!via `Reverse`))

(fn `UserConstructionScript`
  (`PrimitiveComponent.SetMaterial` (`self.SM_Hatch_01_A`) 0 (`self.Material`))
  (`PrimitiveComponent.SetMaterial` (`self.SM_Hatch_01_B`) 0 (`self.Material`)))