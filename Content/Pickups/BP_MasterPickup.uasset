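; Base pickup Blueprint that applies an effect to the first-person player character on touch, then destroys itself.
; When its collider is overlapped, it casts the other actor to BP_FirstPersonCharacter and line traces from its mesh to that character.
; The effect only fires if the trace hits the character, so pickups cannot be collected through blocking objects.
; ApplyPickupEffect is an empty event here, serving as the hook for the specific effect.
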(event `ApplyPickupEffect`
  (params (Player :type "/Game/FirstPerson/Blueprints/BP_FirstPersonCharacter Object Reference")))

(event `self.Collider.OnComponentBeginOverlap`
  (params (OverlappedComponent :type "PrimitiveComponent Object Reference") (OtherActor :type "Actor Object Reference") (OtherComp :type "PrimitiveComponent Object Reference") (OtherBodyIndex :type Integer) (bFromSweep :type Boolean) (SweepResult :type "HitResult Structure (by ref)"))
  (bind _asbp_first_person_character (cast `/Game/FirstPerson/Blueprints/BP_FirstPersonCharacter` OtherActor))
  (bind _outhit (`KismetSystemLibrary.LineTraceSingleForObjects` (`SceneComponent.K2_GetComponentLocation` (`self.StaticMesh`)) (`self.K2_GetActorLocation` _asbp_first_person_character) (`|MakeArray` "ObjectTypeQuery3" "ObjectTypeQuery1" "ObjectTypeQuery2" :!type "EObjectTypeQuery Enum") false (`|MakeArray` self null :!type "Actor Object Reference")))
  (if (== (`.HitActor` (`GameplayStatics.BreakHitResult` _outhit)) _asbp_first_person_character)
    (`self.ApplyPickupEffect` _asbp_first_person_character)
    (`self.K2_DestroyActor`)))

(fn `UserConstructionScript`)