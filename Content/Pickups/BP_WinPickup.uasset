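; BP_WinPickup is a pickup that ends play with a win screen when its effect is applied to the player.
; Its ApplyPickupEffect event clears the player's hover state, fades out the jetpack audio and disables input.
; It then shows the mouse cursor and adds a new WBP_WinScreen widget to the viewport.
; The construction script only calls the parent's version.
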(event `self.ApplyPickupEffect`
  (params (Player :type "/Game/FirstPerson/Blueprints/BP_FirstPersonCharacter Object Reference"))
  (set `/Game/FirstPerson/Blueprints/BP_FirstPersonCharacter.IsHovering` false Player)
  (`AudioComponent.FadeOut` (`/Game/FirstPerson/Blueprints/BP_FirstPersonCharacter.JetpackAudio` Player) 0.1 0.0 "Linear")
  (bind _asplayer_controller (cast `PlayerController` (`Pawn.GetController` Player)))
  (`self.DisableInput` Player _asplayer_controller)
  (set `PlayerController.bShowMouseCursor` true _asplayer_controller)
  (bind _returnvalue (`|CreateWidget` "/Game/UI/WBP_WinScreen.WBP_WinScreen_C"))
  (`UserWidget.AddToViewport` _returnvalue 0))

(fn `UserConstructionScript`
  (`parent.UserConstructionScript`))