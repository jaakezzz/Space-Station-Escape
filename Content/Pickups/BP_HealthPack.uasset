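; Health pack pickup that restores a player's health through the ApplyPickupEffect event.
; It adds HealAmount to the player's CurrentHealth, clamped between zero and MaxHealth.
; It then prints the new health value and plays the pickup sound at the player's location.
; The construction script only calls its parent, and the event graph contains no trigger or removal logic of its own.
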(event `self.ApplyPickupEffect`
  (params (Player :type "/Game/FirstPerson/Blueprints/BP_FirstPersonCharacter Object Reference"))
  (bind _currenthealth (`/Game/FirstPerson/Blueprints/BP_FirstPersonCharacter.CurrentHealth` Player))
  (set `/Game/FirstPerson/Blueprints/BP_FirstPersonCharacter.CurrentHealth` (`KismetMathLibrary.FClamp` (+ _currenthealth (`self.HealAmount`)) 0.0 (`/Game/FirstPerson/Blueprints/BP_FirstPersonCharacter.MaxHealth` Player)) Player)
  (`KismetSystemLibrary.PrintString` (`KismetStringLibrary.Conv_DoubleToString` _currenthealth))
  (`GameplayStatics.PlaySoundAtLocation` "/Game/Audio/SFX/pickup-health.pickup-health" (`SceneComponent.K2_GetComponentLocation` (`Actor.RootComponent` Player)) (struct) 0.5 1.0 0.0 null null null null))

(fn `UserConstructionScript`
  (`parent.UserConstructionScript`))